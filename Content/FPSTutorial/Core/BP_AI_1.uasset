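; Melee enemy AI character that chases the player and plays an attack montage when close.
; PawnSensing sightings set a seen flag and re-issue an AI MoveTo toward player 0; Tick halts movement while the flag is unset.
; Reaching the player plays a counter-attack montage, gated by CanAttack and a delay of the montage's length.
; AnyDamage reduces health, switching to ragdoll physics and disabling movement at zero.
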(event OnSeePawn(PawnSensing)
  (params (Pawn :type Pawn%20Object%20Reference))
  (Variables|Default|SetisSeenPlayer true)
  (CallFunction|FollowPlayer))

(event Custom|FollowPlayer
  (Variables|Default|SetcanAttack true)
  (if (Variables|Default|GetisSeenPlayer)
    (AI|AIMoveTo self "0, 0, 0" (Game|GetPlayerCharacter 0) 1.5e+02 false
      (:OnSuccess
        (if (Variables|Default|GetcanAttack)
          (Variables|Default|SetcanAttack false)
          (bind _returnvalue (Animation|PlayAnimMontage "/Game/FreeAnimationLibrary/Animations/Counter-Finisher/AM_anim_Counter_Attack_08_Montage.AM_anim_Counter_Attack_08_Montage" 1.0 "None"))
          (Utilities|FlowControl|Delay _returnvalue)
          (Variables|Default|SetcanAttack true))))
    (else
      (Variables|Default|SetisSeenPlayer false))))

(event EventBeginPlay)

(event Collision|EventActorBeginOverlap
  (params (OtherActor :type Actor%20Object%20Reference)))

(event EventTick
  (params (DeltaSeconds :type Float%20%28single-precision%29))
  (if (not (Variables|Default|GetisSeenPlayer))
    (Components|Movement|StopMovementImmediately (Variables|Character|GetCharacterMovement))))

(event Game|Damage|EventAnyDamage
  (params (Damage :type Float%20%28single-precision%29) (DamageType :type Damage%20Type%20Object%20Reference) (InstigatedBy :type Controller%20Object%20Reference) (DamageCauser :type Actor%20Object%20Reference))
  (Variables|Default|SetcurrentHealth (- (Variables|Default|GetcurrentHealth) Damage))
  (if (<= (Variables|Default|GetcurrentHealth) 0.0)
    (Physics|SetSimulatePhysics (Variables|Character|GetMesh) true)
    (Pawn|Components|CharacterMovement|SetMovementMode (Variables|Character|GetCharacterMovement) "MOVE_None" 0)))

(fn ConstructionScript)