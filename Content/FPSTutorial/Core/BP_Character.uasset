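; First-person shooter player character that handles Enhanced Input movement, look, jump, timeline-driven sprint FOV and crouch, aiming state, and weapon actions.
; On BeginPlay it spawns Inventory weapons onto the arms' hand socket, shows the selected one and creates the HUD.
; Firing loops through a delay while held, spawning bullets from the camera and triggering weapon messages and montages.
; A per-tick camera trace blocks firing near walls, alongside running, reload, ammo and holster checks.
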(event Custom|StoppRunning
  ;[0.15 0.15 0.15 0.5] Running
  (Variables|Default|SetisRunning false)
  (Variables|/Script/Engine.CharacterMovementComponent|SetMaxWalkSpeed (Variables|Character|GetCharacterMovement) 6e+02)
  (bind _fov (Timeline|时间轴 ReverseFromEnd)
    (:Update
      (Variables|/Script/Engine.PlayerCameraManager|SetDefaultFOV (Game|GetPlayerCameraManager 0) _fov))))

(event Custom|Custom%20Uncrouch
  (Variables|Default|SetisCrouching false)
  (Variables|/Script/Engine.CharacterMovementComponent|SetMaxWalkSpeed (Variables|Character|GetCharacterMovement) 6e+02)
  (bind _half_height (Timeline|Crouch%20Timeline Reverse)
    (:Update
      (Components|Capsule|SetCapsuleHalfHeight (Variables|Collision|GetCapsuleComponent) _half_height true))))

(event Custom|Custom%20Crouch
  (Variables|Default|SetisCrouching true)
  (CallFunction|StoppRunning)
  (Variables|/Script/Engine.CharacterMovementComponent|SetMaxWalkSpeed (Variables|Character|GetCharacterMovement) 4e+02)
  (bind _half_height (Timeline|Crouch%20Timeline Play)
    (:Update
      (Components|Capsule|SetCapsuleHalfHeight (Variables|Collision|GetCapsuleComponent) _half_height true))))

(event Custom|ToggleHolster
  (Variables|Default|SetisEquipped (not (Variables|Default|GetisEquipped)))
  (Animation|Montage|PlayMontage (Variables|Default|GetCharacterArms) (select (Variables|Default|GetisEquipped) "/Game/FPSTutorial/Art/AssaultRifle/Animations/AM_FP_AssaultRifle_Equip.AM_FP_AssaultRifle_Equip" "/Game/FPSTutorial/Art/AssaultRifle/Animations/AM_FP_AssaultRifle_Holster.AM_FP_AssaultRifle_Holster")))

(event Input|EnhancedActionEvents|EnhancedInputActionIA_Camera
  (params (ActionValue :type Vector%202D%20Structure) (ElapsedSeconds :type Float%20%28double-precision%29) (TriggeredSeconds :type Float%20%28double-precision%29) (InputAction :type Input%20Action%20Object%20Reference :default "/Game/FPSTutorial/Data/IA_Camera.IA_Camera"))
  ;[0.15 0.15 0.15 0.5] Camera
  (:Triggered
    (Variables|Default|SetmouseInput ActionValue :!label _label)
    (Pawn|Input|AddControllerPitchInput (* (.Y (Math|Vector2D|BreakVector2D (Variables|Default|GetmouseInput))) -1.0))
    (Pawn|Input|AddControllerYawInput (.X (Math|Vector2D|BreakVector2D (Variables|Default|GetmouseInput)))))
  (:Completed
    (goto _label)))

(event Input|EnhancedActionEvents|EnhancedInputActionIA_Shoot
  (params (ActionValue :type Boolean) (ElapsedSeconds :type Float%20%28double-precision%29) (TriggeredSeconds :type Float%20%28double-precision%29) (InputAction :type Input%20Action%20Object%20Reference :default "/Game/FPSTutorial/Data/IA_Shoot.IA_Shoot"))
  (:Triggered
    (Utilities|FlowControl|DoOnce false :!label _label
      (:Completed
        (Variables|Default|SetisHoldShooting true)
        ;[0.15 0.15 0.15 0.5] Fire
        (if (and (and (and (Math|Boolean|ANDBoolean (Variables|Default|GetisHoldShooting) (not (Variables|Default|GetisRunning)) (not (Variables|Default|GetisCloseToWall))) (> (Variables|Default|GetcurrentAmmo) 0)) (not (Variables|Default|GetisReloading))) (Variables|Default|GetisEquipped)) :!label _label_2
          (Class|BPIWeapon|Shoot(Message) (Utilities|Array|Get(acopy) (Variables|Default|GetEquippedWeapons) (Variables|Default|GetEquippedWeaponIndex)))
          (Animation|Montage|PlayMontage (Variables|Default|GetCharacterArms) "/Game/FPSTutorial/Art/AssaultRifle/Animations/AM_FP_AssaultRifle_Fire.AM_FP_AssaultRifle_Fire"
            (:then
              (bind _returnvalue (Game|SpawnActorfromClass "/Game/FPSTutorial/Core/BP_Bullet.BP_Bullet_C" (Transformation|GetWorldTransform (Variables|Default|GetCamera)) "AlwaysSpawn" "MultiplyWithRoot" 0 0))
              (Collision|IgnoreActorwhenMoving (Variables|Collision|GetCapsuleComponent) _returnvalue false)
              (Collision|IgnoreActorwhenMoving (Variables|/Game/FPSTutorial/Core/BP_Bullet.BP_Bullet_C|GetSphere _returnvalue) self true)
              (Effects|SpawnEmitterAttached "/Game/StarterContent/Particles/P_Explosion.P_Explosion" (Variables|/Script/Engine.Actor|GetRootComponent (Utilities|Array|Get(acopy) (Variables|Default|GetEquippedWeapons) (Variables|Default|GetEquippedWeaponIndex))) "None" "0.000000,100.000000,0.000000" "0, 0, 0" "0.050000,0.050000,0.050000" "SnapToTargetIncludingScale")
              (Variables|Default|SetcurrentAmmo (- (Variables|Default|GetcurrentAmmo) 1))
              (Utilities|FlowControl|Delay (Variables|Default|GetfireDelay))
              (goto _label_2)))))))
  (:Completed
    (Variables|Default|SetisHoldShooting false)
    (goto _label Reset)))

(event Input|EnhancedActionEvents|EnhancedInputActionIA_Movement
  (params (ActionValue :type Vector%202D%20Structure) (ElapsedSeconds :type Float%20%28double-precision%29) (TriggeredSeconds :type Float%20%28double-precision%29) (InputAction :type Input%20Action%20Object%20Reference :default "/Game/FPSTutorial/Data/IA_Movement.IA_Movement"))
  ;[0.15 0.15 0.15 0.5] Movement
  (:Triggered
    (Variables|Default|SetmoveInput ActionValue :!label _label)
    (Pawn|Input|AddMovementInput (* (Transformation|GetActorForwardVector) (.Y (Math|Vector2D|BreakVector2D (Variables|Default|GetmoveInput)))) 1.0 false)
    (Pawn|Input|AddMovementInput (* (Transformation|GetActorRightVector) (.X (Math|Vector2D|BreakVector2D (Variables|Default|GetmoveInput)))) 1.0 false))
  (:Completed
    (goto _label)))

(event Input|EnhancedActionEvents|EnhancedInputActionIA_Run
  (params (ActionValue :type Boolean) (ElapsedSeconds :type Float%20%28double-precision%29) (TriggeredSeconds :type Float%20%28double-precision%29) (InputAction :type Input%20Action%20Object%20Reference :default "/Game/FPSTutorial/Data/IA_Run.IA_Run"))
  ;[0.15 0.15 0.15 0.5] Running
  (:Triggered
    (if (not (AI|Components|NavMovement|IsFalling (Variables|Character|GetCharacterMovement)))
      (if (not (Variables|Default|GetisCrouching))
        (Variables|Default|SetisRunning true)
        (Variables|/Script/Engine.CharacterMovementComponent|SetMaxWalkSpeed (Variables|Character|GetCharacterMovement) (Variables|Default|GetrunningSpeed))
        (bind _fov (Timeline|时间轴 Play)
          (:Update
            (Variables|/Script/Engine.PlayerCameraManager|SetDefaultFOV (Game|GetPlayerCameraManager 0) _fov))))))
  (:Completed
    (CallFunction|StoppRunning)))

(event Input|EnhancedActionEvents|EnhancedInputActionIA_Jump
  (params (ActionValue :type Boolean) (ElapsedSeconds :type Float%20%28double-precision%29) (TriggeredSeconds :type Float%20%28double-precision%29) (InputAction :type Input%20Action%20Object%20Reference :default "/Game/FPSTutorial/Data/IA_Jump.IA_Jump"))
  (:Triggered
    (Character|Jump)
    (CallFunction|StoppRunning))
  (:Completed
    (Character|StopJumping)))

(event Input|EnhancedActionEvents|EnhancedInputActionIA_Crouch
  (params (ActionValue :type Boolean) (ElapsedSeconds :type Float%20%28double-precision%29) (TriggeredSeconds :type Float%20%28double-precision%29) (InputAction :type Input%20Action%20Object%20Reference :default "/Game/FPSTutorial/Data/IA_Crouch.IA_Crouch"))
  ;[0.15 0.15 0.15 0.5] Crouch
  (:Triggered
    (Utilities|FlowControl|DoOnce false :!label _label
      (:Completed
        (if (Variables|Default|GetholdCrouch)
          (CallFunction|CustomCrouch)
          (else
            (Utilities|FlowControl|FlipFlop
              (:A
                (CallFunction|CustomCrouch))
              (:B
                (CallFunction|CustomUncrouch))))))))
  (:Completed
    (if (Variables|Default|GetholdCrouch)
      (CallFunction|CustomUncrouch)
      (goto _label Reset)
      (else
        (goto _label Reset)))))

(event Input|EnhancedActionEvents|EnhancedInputActionIA_Aim
  (params (ActionValue :type Boolean) (ElapsedSeconds :type Float%20%28double-precision%29) (TriggeredSeconds :type Float%20%28double-precision%29) (InputAction :type Input%20Action%20Object%20Reference :default "/Game/FPSTutorial/Data/IA_Aim.IA_Aim"))
  ;[0.15 0.15 0.15 0.5] Aiming System
  (:Triggered
    (Variables|Default|SetisAiming true))
  (:Completed
    (Variables|Default|SetisAiming false)))

(event Input|EnhancedActionEvents|EnhancedInputActionIA_Reload
  (params (ActionValue :type Boolean) (ElapsedSeconds :type Float%20%28double-precision%29) (TriggeredSeconds :type Float%20%28double-precision%29) (InputAction :type Input%20Action%20Object%20Reference :default "/Game/FPSTutorial/Data/IA_Reload.IA_Reload"))
  ;[0.15 0.15 0.15 0.5] Reload
  (:Triggered
    (Utilities|FlowControl|DoOnce false :!label _label
      (:Completed
        (if (Variables|Default|GetisEquipped)
          (Variables|Default|SetisReloading true)
          (Animation|Montage|PlayMontage (Variables|Default|GetCharacterArms) "/Game/FPSTutorial/Art/AssaultRifle/Animations/AM_FP_AssaultRifle_Reload.AM_FP_AssaultRifle_Reload"
            (:then
              (Class|BPIWeapon|Reload(Message) (Utilities|Array|Get(acopy) (Variables|Default|GetEquippedWeapons) (Variables|Default|GetEquippedWeaponIndex)))
              (Utilities|FlowControl|Delay 1.9)
              (Variables|Default|SetcurrentAmmo (Variables|Default|GettotalAmmo)))
            (:OnBlendOut
              (Variables|Default|SetisReloading false)))))))
  (:Completed
    (goto _label Reset)))

(event Input|EnhancedActionEvents|EnhancedInputActionIA_Holster
  (params (ActionValue :type Boolean) (ElapsedSeconds :type Float%20%28double-precision%29) (TriggeredSeconds :type Float%20%28double-precision%29) (InputAction :type Input%20Action%20Object%20Reference :default "/Game/FPSTutorial/Data/IA_Holster.IA_Holster"))
  (:Triggered
    (Utilities|FlowControl|DoOnce false :!label _label
      (:Completed
        (Variables|Default|SetisEquipped (not (Variables|Default|GetisEquipped)))
        (Animation|Montage|PlayMontage (Variables|Default|GetCharacterArms) (select (Variables|Default|GetisEquipped) "/Game/FPSTutorial/Art/AssaultRifle/Animations/AM_FP_AssaultRifle_Equip.AM_FP_AssaultRifle_Equip" "/Game/FPSTutorial/Art/AssaultRifle/Animations/AM_FP_AssaultRifle_Holster.AM_FP_AssaultRifle_Holster")))))
  (:Completed
    (goto _label Reset)))

(event EventTick
  (params (DeltaSeconds :type Float%20%28single-precision%29))
  (bind _camera (Variables|Default|GetCamera))
  ;[0.15 0.15 0.15 0.5] Event Tick
  (Transformation|SetRelativeRotation (Variables|Default|GetPivot) (Math|Rotator|MakeRotator 0.0 (.Pitch (Math|Rotator|BreakRotator (Pawn|GetControlRotation :!class /Script/Engine.Pawn))) 0.0) false false)
  (bind _returnvalue (Collision|LineTraceByChannel (Transformation|GetWorldLocation (Variables|Default|GetCamera)) (+ (Transformation|GetWorldLocation _camera) (* (Math|Vector|GetForwardVector _camera) "100.000000,100.000000,100.000000")) "TraceTypeQuery1" false 0 "None"))
  (Variables|Default|SetisCloseToWall _returnvalue))

(event EventBeginPlay
  (Input|AddMappingContext (PlayerController|LocalPlayerSubsystems|GetEnhancedInputLocalPlayerSubsystem (Game|GetPlayerController 0)) "/Game/FPSTutorial/Data/IMC_FPS.IMC_FPS" 0 "(bIgnoreAllPressedKeysUntilRelease=True,bForceImmediately=False,bNotifyUserSettings=False)")
  (CallFunction|SpawnWeapon)
  ;[0.15 0.15 0.15 0.5] Create UI
  (bind _returnvalue (UserInterface|CreateWidget "/Game/FPSTutorial/Core/WBP_UI.WBP_UI_C" (Game|GetPlayerController 0)))
  (UserInterface|Viewport|AddtoViewport _returnvalue 0)
  (CallFunction|ToggleHolster))

(fn ConstructionScript)

(fn SpawnWeapon
  (for _array_element (Variables|Default|GetInventory)
    (bind _returnvalue (Game|SpawnActorfromClass _array_element (Math|Transform|MakeTransform "0, 0, 0" "0, 0, 0" "1.000000,1.000000,1.000000") "Undefined" "MultiplyWithRoot" 0 0))
    (Utilities|Array|Add (Variables|Default|GetEquippedWeapons) _returnvalue)
    (Transformation|AttachComponentToComponent _returnvalue (Variables|Default|GetCharacterArms) "ik_hand_gun" "SnapToTarget" "SnapToTarget" "KeepRelative" true)
    (Rendering|SetActorHiddenInGame _returnvalue true))
  (Rendering|SetActorHiddenInGame (Utilities|Array|Get(acopy) (Variables|Default|GetEquippedWeapons) (Variables|Default|GetEquippedWeaponIndex)) false))